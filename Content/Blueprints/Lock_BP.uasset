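; Lock actor that ends the game when an actor tagged "Unlock3" overlaps its box.
; After a brief delay it destroys that actor, reveals its own key mesh and animates it to the transform of a second key mesh.
; It then shows the EndGameScreen widget, pauses the game and switches input to UI-only with the mouse cursor visible.
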(event `self.Box.OnComponentBeginOverlap`
  (params (OverlappedComponent :type "PrimitiveComponent Object Reference") (OtherActor :type "Actor Object Reference") (OtherComp :type "PrimitiveComponent Object Reference") (OtherBodyIndex :type Integer) (bFromSweep :type Boolean) (SweepResult :type "HitResult Structure (by ref)"))
  (bind _returnvalue (`GameplayStatics.GetPlayerController` 0))
  (bind _sm_lock_key (`self.SM_Lock_Key`))
  (bind _sm_lock_key1 (`self.SM_Lock_Key1`))
  (if (`self.ActorHasTag` OtherActor "Unlock3")
    (`KismetSystemLibrary.Delay` 0.2)
    (`self.K2_DestroyActor` OtherActor)
    (`SceneComponent.SetVisibility` _sm_lock_key true false)
    (`KismetSystemLibrary.MoveComponentTo` _sm_lock_key (`SceneComponent.RelativeLocation` _sm_lock_key1) (`SceneComponent.RelativeRotation` _sm_lock_key1) false false 1.0)
    (bind _returnvalue_2 (`|GenericCreateObject` "/Game/UI_Widgets/EndGameScreen.EndGameScreen_C"))
    (`UserWidget.AddToViewport` _returnvalue_2 0)
    (bind _returnvalue_3 (`GameplayStatics.SetGamePaused` true))
    (set `PlayerController.bShowMouseCursor` _returnvalue_3 _returnvalue)
    (`WidgetBlueprintLibrary.SetInputMode_UIOnlyEx` _returnvalue _returnvalue_2)))

(fn `UserConstructionScript`)