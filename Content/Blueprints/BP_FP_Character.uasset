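; First-person character Blueprint that adds object grabbing, a toggleable light and a pause menu through Enhanced Input actions.
; The grab action calls Grab on the GrabberC component on start and on every trigger, and Release on completion or cancel.
; The light action toggles the SpotLight's visibility.
; Escape creates PauseMenuUI, pauses the game, sets cursor visibility from the pause result and switches input to UI only.
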(event `EnhancedInput|/Game/FirstPerson/Input/Actions/IA_Grab`
  (params (ActionValue :type Boolean) (ElapsedSeconds :type "Float (double-precision)") (TriggeredSeconds :type "Float (double-precision)") (InputAction :type "InputAction Object Reference" :default "/Game/FirstPerson/Input/Actions/IA_Grab.IA_Grab"))
  (bind _grabber_c (`self.Grabber_C`))
  (:`Triggered`
    (`Grabber_C.Grab` _grabber_c :!label _label))
  (:`Started`
    (goto _label))
  (:`Canceled`
    (`Grabber_C.Release` _grabber_c :!label _label_2))
  (:`Completed`
    (goto _label_2)))

(event `EnhancedInput|/Game/FirstPerson/Input/Actions/IA_Light`
  (params (ActionValue :type Boolean) (ElapsedSeconds :type "Float (double-precision)") (TriggeredSeconds :type "Float (double-precision)") (InputAction :type "InputAction Object Reference" :default "/Game/FirstPerson/Input/Actions/IA_Light.IA_Light"))
  (:`Started`
    (`SceneComponent.ToggleVisibility` (`self.SpotLight`) false)))

(event `EnhancedInput|/Game/FirstPerson/Input/Actions/IA_Escape`
  (params (ActionValue :type Boolean) (ElapsedSeconds :type "Float (double-precision)") (TriggeredSeconds :type "Float (double-precision)") (InputAction :type "InputAction Object Reference" :default "/Game/FirstPerson/Input/Actions/IA_Escape.IA_Escape"))
  (bind _returnvalue (`GameplayStatics.GetPlayerController` 0))
  (:`Started`
    (bind _returnvalue_2 (`|GenericCreateObject` "/Game/UI_Widgets/PauseMenuUI.PauseMenuUI_C"))
    (`UserWidget.AddToViewport` _returnvalue_2 0)
    (bind _returnvalue_3 (`GameplayStatics.SetGamePaused` true))
    (set `PlayerController.bShowMouseCursor` _returnvalue_3 _returnvalue)
    (`WidgetBlueprintLibrary.SetInputMode_UIOnlyEx` _returnvalue _returnvalue_2)))

(fn `UserConstructionScript`
  (`parent.UserConstructionScript`))